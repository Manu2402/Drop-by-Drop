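; BP_GeneratorHeightMap builds heightmap terrain when play begins, either procedurally or from a saved PNG, selected by GenerateFromPng.
; In procedural mode it generates height data on the CPU at MapSize, converts it to a texture and saves that as a PNG under Saved/HeightMap.
; It then spawns a HeightMapMeshActor, which builds the mesh from the fresh data or the PNG in that folder, using fixed height and XY scales.
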(event `self.ReceiveBeginPlay`
  (bind _mapsize (`self.MapSize`))
  (if (not (`self.GenerateFromPng`))
    (bind _returnvalue (`self.GenerateHeightMapCPU` _mapsize))
    (bind _returnvalue_2 (`self.CreateHeightMapTexture` _returnvalue _mapsize _mapsize))
    (`self.SaveTextureToFile` _returnvalue_2 (`KismetStringLibrary.Concat_StrStr` (`BlueprintPathsLibrary.ProjectDir`) "Saved/HeightMap/Heightmap.png")))
  (bind _returnvalue_3 (`|SpawnActorFromClass` "/Script/DropbyDrop.HeightMapMeshActor" (`KismetMathLibrary.MakeTransform` (0.0 0.0 0.0)) "Undefined" "MultiplyWithRoot" null null))
  (if (`self.GenerateFromPng`)
    (`HeightMapMeshActor.GenerateMeshFromPng` _returnvalue_3 (`KismetStringLibrary.Concat_StrStr` (`BlueprintPathsLibrary.ProjectDir`) "Saved/HeightMap/HeightMap.png") (`self.MapSize`) 400.0 1.0)
    (else
      (`HeightMapMeshActor.GenerateMeshFromHeightMap` _returnvalue_3 _returnvalue (`self.MapSize`) 400.0 1.0))))

(fn `UserConstructionScript`)